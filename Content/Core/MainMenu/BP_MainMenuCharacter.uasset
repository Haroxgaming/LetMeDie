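; BP_MainMenuCharacter is a character for the main menu that the player can move along one axis and make jump.
; On BeginPlay it adds the IMC_MainMenu Enhanced Input mapping context to the first player controller's subsystem.
; AI_MoveMenu feeds movement along a forward vector built with zeroed pitch and yaw, so it stays on world X regardless of facing.
; AI_JumpMenu starts a jump and stops it on cancel or completion.
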(event Input|EnhancedActionEvents|EnhancedInputActionAI_MoveMenu
  (params (ActionValue :type Vector%202D%20Structure) (ElapsedSeconds :type Float%20%28double-precision%29) (TriggeredSeconds :type Float%20%28double-precision%29) (InputAction :type Input%20Action%20Object%20Reference :default "/Game/Core/MainMenu/Inputs/AI_MoveMenu.AI_MoveMenu"))
  (Pawn|Input|AddMovementInput (Math|Vector|GetForwardVector (Math|Rotator|MakeRotator (.roll (Pawn|GetControlRotation :!class /Script/Engine.Pawn)) 0.0 0.0)) (.x ActionValue) false))

(event Input|EnhancedActionEvents|EnhancedInputActionAI_JumpMenu
  (params (ActionValue :type Boolean) (ElapsedSeconds :type Float%20%28double-precision%29) (TriggeredSeconds :type Float%20%28double-precision%29) (InputAction :type Input%20Action%20Object%20Reference :default "/Game/Core/MainMenu/Inputs/AI_JumpMenu.AI_JumpMenu"))
  (:Started
    (Character|Jump))
  (:Canceled
    (Character|StopJumping :!label _label))
  (:Completed
    (goto _label)))

(event EventBeginPlay
  (bind _returnvalue (Game|GetPlayerController 0))
  (bind _returnvalue_2 (PlayerController|LocalPlayerSubsystems|GetEnhancedInputLocalPlayerSubsystem _returnvalue))
  (Utilities|IsValid _returnvalue_2
    (:Is%20Valid
      (Input|AddMappingContext _returnvalue_2 "/Game/Core/MainMenu/Inputs/IMC_MainMenu.IMC_MainMenu" 0 "(bIgnoreAllPressedKeysUntilRelease=True,bForceImmediately=False,bNotifyUserSettings=False)"))))

(fn ConstructionScript)