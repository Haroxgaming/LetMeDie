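; BP_Void is a kill volume that triggers the first-person character's death when it overlaps the box.
; It sets IsDead and calls Death with a voiceline row chosen by the current death index.
; That index, set by the window and pipes death events, also picks the cleanup: rebuild the window and destroy the spawn button's boxes, or rebuild the pipes death.
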(event OnComponentBeginOverlap(Box)
  (params (OverlappedComponent :type Primitive%20Component%20Object%20Reference) (OtherActor :type Actor%20Object%20Reference) (OtherComp :type Primitive%20Component%20Object%20Reference) (OtherBodyIndex :type Integer) (bFromSweep :type Boolean) (SweepResult :type Hit%20Result%20Structure%20%28by%20ref%29))
  (bind _asbp_first_person_character (Utilities|Casting|CastToBP_FirstPersonCharacter OtherActor))
  (Variables|/Game/FirstPerson/Blueprints/BP_FirstPersonCharacter.BP_FirstPersonCharacter_C|SetIsDead%20? _asbp_first_person_character true)
  (Default|Death _asbp_first_person_character (Utilities|Array|Get(acopy) (Variables|Default|GetVoicelines_Raw) (Variables|Default|Getdeathcurrent)) false)
  (switch int (Variables|Default|Getdeathcurrent)
    (:0
      (Default|Rebuild (Variables|Default|GetWindowRef))
      (Default|DestroyBoxes (Variables|Default|GetSpawnButtonRef)))
    (:1
      (Default|Rebuild (Variables|Default|GetPipesDeathRef)))))

(event Custom|ReceiveWindowDeath
  (Variables|Default|Setdeathcurrent 0))

(event Custom|ReceivePipesDeath
  (Variables|Default|Setdeathcurrent 1))

(fn ConstructionScript)