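; Death trap that triggers when the first-person character grows from small to normal size inside a box around pipes.
; While the player overlaps, a looping timer polls the SmallToNormal timeline, then once turns on pipe physics and notifies VoidRef of the death.
; Rebuild restores the pipe transforms saved at BeginPlay and sets HasDied.
; After that, the box blocks regrowing instead, until shortly after the player leaves.
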(event OnComponentBeginOverlap(Box)
  (params (OverlappedComponent :type Primitive%20Component%20Object%20Reference) (OtherActor :type Actor%20Object%20Reference) (OtherComp :type Primitive%20Component%20Object%20Reference) (OtherBodyIndex :type Integer) (bFromSweep :type Boolean) (SweepResult :type Hit%20Result%20Structure%20%28by%20ref%29))
  (bind _asbp_first_person_character (Utilities|Casting|CastToBP_FirstPersonCharacter OtherActor))
  (bind _output_get (Variables|Default|SetAs%20BP%20First%20Person%20Character _asbp_first_person_character))
  (if (not (Variables|Default|GetbHasDied?))
    (bind _returnvalue (Utilities|Time|SetTimerbyEvent (delegate Custom|CustomEvent) 0.2 true))
    (Variables|Default|SetNewVar _returnvalue)
    (else
      (Variables|/Game/FirstPerson/Blueprints/BP_FirstPersonCharacter.BP_FirstPersonCharacter_C|SetbCantRegrow _output_get true))))

(event OnComponentEndOverlap(Box)
  (params (OverlappedComponent :type Primitive%20Component%20Object%20Reference) (OtherActor :type Actor%20Object%20Reference) (OtherComp :type Primitive%20Component%20Object%20Reference) (OtherBodyIndex :type Integer))
  (bind _asbp_first_person_character (Utilities|Casting|CastToBP_FirstPersonCharacter OtherActor))
  (if (not (Variables|Default|GetbHasDied?))
    (Utilities|Time|ClearandInvalidateTimerbyHandle (Variables|Default|GetNewVar))
    (else
      (Utilities|FlowControl|Delay 1.0)
      (Variables|/Game/FirstPerson/Blueprints/BP_FirstPersonCharacter.BP_FirstPersonCharacter_C|SetbCantRegrow _asbp_first_person_character false))))

(event Custom|CustomEvent
  (if (Audio|Components|Audio|IsPlaying (Variables|/Game/FirstPerson/Blueprints/BP_FirstPersonCharacter.BP_FirstPersonCharacter_C|GetSmallToNormal (Variables|Default|GetPlayerRef)))
    (Utilities|FlowControl|DoOnce false
      (:Completed
        (for _array_element (Variables|Default|GetPipes)
          (Physics|SetSimulatePhysics (Variables|/Script/Engine.StaticMeshActor|GetStaticMeshComponent _array_element) true))
        (Default|ReceivePipesDeath (Variables|Default|GetVoidRef))
        (Utilities|Time|ClearandInvalidateTimerbyHandle (Variables|Default|GetNewVar))))))

(event Custom|Rebuild
  (for (_array_element _array_index) (Variables|Default|GetPipes)
    (Physics|SetSimulatePhysics (Variables|/Script/Engine.StaticMeshActor|GetStaticMeshComponent _array_element) false)
    (Transformation|SetActorTransform _array_element (Utilities|Array|Get(acopy) (Variables|Default|GetLocRefs) _array_index)))
  (Variables|Default|SetbHasDied? true))

(event EventBeginPlay
  (|CallParentFunction)
  (for _array_element (Variables|Default|GetPipes)
    (Utilities|Array|Add (Variables|Default|GetLocRefs) (Transformation|GetActorTransform _array_element))))

(event Collision|EventActorBeginOverlap
  (params (OtherActor :type Actor%20Object%20Reference)))

(event EventTick
  (params (DeltaSeconds :type Float%20%28single-precision%29)))

(fn ConstructionScript
  (|CallParentFunction))