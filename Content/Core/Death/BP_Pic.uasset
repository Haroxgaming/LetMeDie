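; Spike hazard that kills the first-person character on overlap, with a death voiceline that advances with each death.
; Once its death counter reaches two, the next overlap instead destroys the spikes, changes BPReset visibility, sets a point light's intensity and plays a "SpikesRemoved" subtitle.
; On BeginPlay it binds its destroy event to the PicHide dispatcher of the BP_Pic returned by GetActorOfClass.
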(event OnComponentBeginOverlap(Box)
  (params (OverlappedComponent :type Primitive%20Component%20Object%20Reference) (OtherActor :type Actor%20Object%20Reference) (OtherComp :type Primitive%20Component%20Object%20Reference) (OtherBodyIndex :type Integer) (bFromSweep :type Boolean) (SweepResult :type Hit%20Result%20Structure%20%28by%20ref%29))
  (Utilities|Casting|CastToBP_FirstPersonCharacter OtherActor)
  (if (>= (Variables|Default|GetDeathNumber) 2)
    (CallFunction|HideEvent)
    (Default|ChangeVisibility (Variables|Default|GetBP_reset))
    (Rendering|Components|Light|SetIntensity (Variables|/Script/Engine.Light|GetLightComponent (Variables|Default|GetPointLight)) 5e+03)
    (Default|DialogueAnimation (Variables|/Game/FirstPerson/Blueprints/BP_FirstPersonCharacter.BP_FirstPersonCharacter_C|GetSubtitleRef (Variables|Default|GetPlayerRef)) "SpikesRemoved" 1.0)
    (else
      (CallFunction|KillEvent))))

(event Custom|HideEvent
  (Actor|DestroyActor))

(event EventBeginPlay
  (bind _returnvalue (Actor|GetActorOfClass "BP_Pic_C"))
  (EventDispatchers|BindEventtoPicHide _returnvalue (delegate Custom|HideEvent))
  (|CallParentFunction))

(event EventKillEvent
  (bind _deathnumber (Variables|Default|GetDeathNumber))
  (Default|Death (Variables|Default|GetPlayerRef) (Utilities|Array|Get(acopy) (Variables|Default|GetDeathRowArray) _deathnumber) false 1.0 1.0)
  (Math|Integer|IncrementInt _deathnumber))

(fn ConstructionScript
  (|CallParentFunction))