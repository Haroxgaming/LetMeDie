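; Laser hazard that sphere-traces forward from its arrow every tick, reacting to Classic Boxes and the first-person player.
; A blocking box drives a DoOnce-gated timer and timeline that raise material glow, cleared when the box changes or leaves.
; The timer's KillPlayer event only prints "dead" if the player is within KillRadius of the box.
; A direct player hit calls Death, or teleports to checkpoint with one-time subtitles when health is locked or BhasDiedLaser is set.
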(event Custom|KillPlayer
  (if (<= (Transformation|GetDistanceTo (Game|Player|GetPlayerPawn 0) (Variables|Default|GetBP_Box)) (Variables|Default|GetKillRadius))
    (Development|PrintString "dead" true false)))

(event EventTick
  (params (DeltaSeconds :type Float%20%28single-precision%29))
  (bind _arrow (Variables|Default|GetArrow))
  (bind _returnvalue (Transformation|GetWorldLocation _arrow))
  (bind _outhit (Collision|SphereTraceByChannel _returnvalue (+ _returnvalue (* (Math|Vector|GetForwardVector (Variables|Default|GetArrow)) 1.5e+03)) 1e+01 "TraceTypeQuery1" false (Variables|Default|GetActors%20to%20Ignore) "Persistent" true "(R=0.000000,G=0.102712,B=1.000000,A=1.000000)"))
  (bind _asbp_classic_box (Utilities|Casting|CastToBP_ClassicBox (.HitActor (Collision|BreakHitResult _outhit)))
    (:then
      (bind _bp_box (Variables|Default|GetBP_Box)
        (:then
          (if (!= _asbp_classic_box _bp_box)
            (Utilities|Time|ClearandInvalidateTimerbyHandle (Variables|Default|GetNewVar))
            (Audio|Components|Audio|Stop (Variables|Default|GetCubeFeedback))
            (Rendering|Material|SetScalarParameterValueonMaterials (Variables|/Game/Core/ClassicObject/BP_ClassicBox.BP_ClassicBox_C|GetStaticMesh _bp_box) "Alpha" 0.0)
            (Rendering|Material|SetScalarParameterValueonMaterials (Variables|/Game/Core/ClassicObject/BP_ClassicBox.BP_ClassicBox_C|GetStaticMesh _bp_box) "StrongerEmissive" 0.0)
            (Utilities|FlowControl|Sequence
              (:then_0
                (goto _label Reset))
              (:then_1
                _))))
        (:else
          _))
      (Utilities|FlowControl|Sequence
        (:then_0
          (Variables|Default|SetBP_Box _asbp_classic_box)
          (Utilities|FlowControl|DoOnce false :!label _label
            (:Completed
              (Utilities|FlowControl|Sequence
                (:then_0
                  (bind _returnvalue_2 (Utilities|Time|SetTimerbyEvent (delegate Custom|KillPlayer) 8.0))
                  (Variables|Default|SetNewVar _returnvalue_2))
                (:then_1
                  (bind (_direction _lerpmat _intensity) (Timeline|CubeFeedback PlayFromStart)
                    (:Update
                      (Rendering|Material|SetScalarParameterValueonMaterials (Variables|/Game/Core/ClassicObject/BP_ClassicBox.BP_ClassicBox_C|GetStaticMesh (Variables|Default|GetBP_Box)) "Alpha" (Math|Float|Lerp 0.0 1.0 _lerpmat))
                      (Rendering|Material|SetScalarParameterValueonMaterials (Variables|/Game/Core/ClassicObject/BP_ClassicBox.BP_ClassicBox_C|GetStaticMesh (Variables|Default|GetBP_Box)) "StrongerEmissive" (Math|Float|Lerp 1.0 2.0 _intensity)))))))))
        (:then_1
          (goto _label_2 Reset))))
    (:CastFailed
      (Utilities|FlowControl|Sequence
        (:then_0
          (Utilities|FlowControl|DoOnce false :!label _label_2
            (:Completed
              (Utilities|Time|ClearandInvalidateTimerbyHandle (Variables|Default|GetNewVar))
              (Audio|Components|Audio|Stop (Variables|Default|GetCubeFeedback))
              (bind _bp_box_2 (Variables|Default|GetBP_Box)
                (:then
                  (Rendering|Material|SetScalarParameterValueonMaterials (Variables|/Game/Core/ClassicObject/BP_ClassicBox.BP_ClassicBox_C|GetStaticMesh _bp_box_2) "Alpha" 0.0)
                  (Rendering|Material|SetScalarParameterValueonMaterials (Variables|/Game/Core/ClassicObject/BP_ClassicBox.BP_ClassicBox_C|GetStaticMesh _bp_box_2) "StrongerEmissive" 0.0)
                  (goto _label Reset))
                (:else
                  (Development|PrintString "invalid box" true false))))))
        (:then_1
          (Variables|Default|SetBP_Box 0)
          (bind _asbp_first_person_character (Utilities|Casting|CastToBP_FirstPersonCharacter (.HitActor (Collision|BreakHitResult _outhit))))
          (if (and (not (Variables|/Game/FirstPerson/Blueprints/BP_FirstPersonCharacter.BP_FirstPersonCharacter_C|GetbHasLockedHealth? _asbp_first_person_character)) (not (Variables|Default|GetbhasDiedLaser)))
            (Default|Death _asbp_first_person_character (Variables|Default|GetKillLaserHit) false)
            (else
              (Transformation|SetActorLocation _asbp_first_person_character (Variables|/Game/FirstPerson/Blueprints/BP_FirstPersonCharacter.BP_FirstPersonCharacter_C|GetCheckpoint _asbp_first_person_character) false false)
              (if (Variables|/Game/FirstPerson/Blueprints/BP_FirstPersonCharacter.BP_FirstPersonCharacter_C|GetbHasLockedHealth? _asbp_first_person_character)
                (Utilities|FlowControl|DoOnce false
                  (:Completed
                    (Default|DialogueAnimation (Variables|/Game/FirstPerson/Blueprints/BP_FirstPersonCharacter.BP_FirstPersonCharacter_C|GetSubtitleRef _asbp_first_person_character) (Variables|Default|GetLockedHealthLaserHit) 0.0)))
                (elif (Variables|Default|GetbhasDiedLaser)
                  (Utilities|FlowControl|DoOnce false
                    (:Completed
                      (Default|DialogueAnimation (Variables|/Game/FirstPerson/Blueprints/BP_FirstPersonCharacter.BP_FirstPersonCharacter_C|GetSubtitleRef _asbp_first_person_character) (Variables|Default|GetAlreadyDeadLaserHit) 0.0))))))))))))

(fn ConstructionScript)