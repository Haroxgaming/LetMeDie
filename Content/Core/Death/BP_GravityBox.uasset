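; Physics box the player can grab, which kills them if it hits while moving fast vertically.
; Interaction toggles a PhysicsHandle grab, ignoring Pawn collision while held.
; An overlap with high vertical speed kills only while StopAttack is set, which BeginPlay clears after a short delay.
; A kill records the death cause, plays a subtitle and has BP_SpawnButton destroy its boxes.
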(event OnComponentBeginOverlap(Box)
  (params (OverlappedComponent :type Primitive%20Component%20Object%20Reference) (OtherActor :type Actor%20Object%20Reference) (OtherComp :type Primitive%20Component%20Object%20Reference) (OtherBodyIndex :type Integer) (bFromSweep :type Boolean) (SweepResult :type Hit%20Result%20Structure%20%28by%20ref%29))
  (Utilities|Casting|CastToBP_FirstPersonCharacter OtherActor)
  (if (and (> (Math|Float|Absolute(Float) (.z (Transformation|GetVelocity))) 3e+02) (Variables|Default|GetStop%20attack))
    (CallFunction|KillEvent)
    (bind _returnvalue (Actor|GetActorOfClass "/Game/Core/ClassicObject/BP_SpawnButton.BP_SpawnButton_C"))
    (Variables|/Game/Core/ClassicObject/BP_SpawnButton.BP_SpawnButton_C|SetDeath%20? _returnvalue true)
    (Default|DestroyBoxes _returnvalue)))

(event EventBeginPlay
  (|CallParentFunction)
  (Utilities|FlowControl|Delay 1.5)
  (Variables|Default|SetStop%20attack false))

(event EventInteraction
  (params (PlayerRef :type BP%20First%20Person%20Character%20Object%20Reference))
  (bind _staticmesh (Variables|Default|GetStaticMesh))
  (if (Variables|Default|GetGrab)
    (Variables|Default|SetGrab false)
    (Variables|/Game/FirstPerson/Blueprints/BP_FirstPersonCharacter.BP_FirstPersonCharacter_C|SetGrabbing (Variables|Default|GetPlayerRef) false)
    (Physics|Components|PhysicsHandle|ReleaseComponent (Variables|/Game/FirstPerson/Blueprints/BP_FirstPersonCharacter.BP_FirstPersonCharacter_C|GetPhysicsHandle (Variables|Default|GetPlayerRef)))
    (Collision|SetCollisionResponsetoChannel _staticmesh "ECC_Pawn" "ECR_Block")
    (else
      (Variables|Default|SetGrab true)
      (Variables|/Game/FirstPerson/Blueprints/BP_FirstPersonCharacter.BP_FirstPersonCharacter_C|SetGrabbing (Variables|Default|GetPlayerRef) true)
      (Class|PhysicsHandleComponent|GrabComponentatLocation (Variables|/Game/FirstPerson/Blueprints/BP_FirstPersonCharacter.BP_FirstPersonCharacter_C|GetPhysicsHandle (Variables|Default|GetPlayerRef)) (Variables|Default|GetBox) "Scene" (Transformation|GetActorLocation))
      (Collision|SetCollisionResponsetoChannel _staticmesh "ECC_Pawn" "ECR_Ignore"))))

(event EventKillEvent
  (Default|Death (Variables|Default|GetPlayerRef) "None" false)
  (Utilities|Map|Add (Variables|/Game/Core/Narrator/BP_LevelChanger.BP_LevelChanger_C|GetDeathCause (Variables|Default|GetLevelChangerRef)) "NewEnumerator1" true)
  (Default|DialogueAnimation (Variables|Default|GetSubtitle%20Ref) "BoxDeath"))

(fn ConstructionScript
  (|CallParentFunction))