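; BP_SpawnButton is an interactable button that replaces its BP_ClassicBox actors with fresh ones above referenced spawn locations.
; Interaction destroys the previous boxes, then spawns new ones linked back to the button, using the Death flag to raise spawn height and notify the first-person character.
; The Size timeline grows the first three boxes from zero to target scale, then enables physics on all of them.
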(event Custom|destroyBoxes
  (bind _classicboxref (Variables|Default|GetClassicBoxRef))
  (for _array_element _classicboxref
    (Actor|DestroyActor _array_element))
  (Utilities|Array|Clear _classicboxref))

(event EventBeginPlay
  (Components|Timeline|SetPlayRate (Variables|Default|GetSize) (/ 1.0 (Variables|Default|GetSizePlayRate%28s%29))))

(event EventInteraction
  (params (PlayerRef :type BP%20First%20Person%20Character%20Object%20Reference))
  (bind _death__ (Variables|Default|GetDeath%20?))
  (CallFunction|DestroyBoxes)
  (for _index (range 0 (- (Utilities|Array|Length (Variables|Default|GetSpawnLocationRef)) 1))
    (bind _returnvalue (Game|SpawnActorfromClass "/Game/Core/ClassicObject/BP_ClassicBox.BP_ClassicBox_C" (Math|Transform|MakeTransform (Math|Vector|MakeVector (.X (Math|Vector|BreakVector (Transformation|GetActorLocation (Utilities|Array|Get(acopy) (Variables|Default|GetSpawnLocationRef) _index)))) (.Y (Math|Vector|BreakVector (Transformation|GetActorLocation (Utilities|Array|Get(acopy) (Variables|Default|GetSpawnLocationRef) _index)))) (+ (.Z (Math|Vector|BreakVector (Transformation|GetActorLocation (Utilities|Array|Get(acopy) (Variables|Default|GetSpawnLocationRef) _index)))) (Math|Float|SelectFloat 7e+01 6e+02 _death__))) "0, 0, 0" (Variables|Default|GetScale)) "AdjustIfPossibleButAlwaysSpawn" "MultiplyWithRoot" 0 _death__ self 0))
    (Utilities|Array|Add (Variables|Default|GetClassicBoxRef) _returnvalue)
    (if (Variables|Default|GetDeath%20?)
      (Default|BoxButton (.AsBP%20First%20Person%20Character (Utilities|Casting|CastToBP_FirstPersonCharacter (Game|Player|GetPlayerPawn 0))))))
  (bind _alpha (Timeline|Size PlayFromStart)
    (:Update
      (Transformation|SetActorScale3D (Utilities|Array|Get(acopy) (Variables|Default|GetClassicBoxRef)) (Math|Vector|Lerp(Vector) "0, 0, 0" (Variables|Default|GetScale) _alpha)))
    (:Finished
      (for _array_element (Variables|Default|GetClassicBoxRef)
        (Physics|SetSimulatePhysics (Variables|/Game/Core/Death/BP_DeathCauseParent.BP_DeathCauseParent_C|GetBox _array_element) true)))))

(fn ConstructionScript)