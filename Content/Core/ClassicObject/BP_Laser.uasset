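; Laser hazard that kills the first-person player on overlap unless it is blocked or health is locked.
; A BP_ClassicBox in the beam blocks it, shortens the Niagara beam and heats up through timeline-driven emissive material parameters.
; Completed heating destroys any held object and kills the player with an explosion voiceline; removing the box resets beam and glow.
; Separate laser and explosion death flags propagate to every BP_Laser to prevent repeats.
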(event OnComponentBeginOverlap(Box)
  (params (OverlappedComponent :type Primitive%20Component%20Object%20Reference) (OtherActor :type Actor%20Object%20Reference) (OtherComp :type Primitive%20Component%20Object%20Reference) (OtherBodyIndex :type Integer) (bFromSweep :type Boolean) (SweepResult :type Hit%20Result%20Structure%20%28by%20ref%29))
  (bind _asbp_first_person_character (Utilities|Casting|CastToBP_FirstPersonCharacter OtherActor)
    (:then
      (if (Math|Boolean|ANDBoolean (not (Variables|Default|GetbhasDiedLaser?)) (not (Variables|/Game/FirstPerson/Blueprints/BP_FirstPersonCharacter.BP_FirstPersonCharacter_C|GetbHasLockedHealth? _asbp_first_person_character)) (not (Variables|Default|GetbIsBlocked)))
        (Default|Death _asbp_first_person_character (Variables|Default|GetVoiceline%20Row%20Name) false)
        (bind _outactors (Actor|GetAllActorsOfClass "BP_Laser_C"))
        (for _array_element _outactors
          (Variables|BP_Laser_C|SetbhasDiedLaser? _array_element true))))
    (:CastFailed
      (bind _asbp_classic_box (Utilities|Casting|CastToBP_ClassicBox OtherActor))
      (Development|PrintString "box in col")
      (Variables|Default|SetbIsBlocked true)
      (Niagara|SetNiagaraVariable(Vector3) (Variables|Default|GetNiagara) "Beam Start" (Math|Vector|MakeVector (Math|Vector|Distance(Vector) (Transformation|GetWorldLocation (Variables|/Game/Core/ClassicObject/BP_ClassicBox.BP_ClassicBox_C|GetStaticMesh _asbp_classic_box)) (Transformation|GetWorldLocation (Variables|Default|GetStartBeam))) 0.0 0.0))
      (if (not (Variables|Default|GetbhasDiedExplosion?))
        (CallFunction|Heat)))))

(event OnComponentEndOverlap(Box)
  (params (OverlappedComponent :type Primitive%20Component%20Object%20Reference) (OtherActor :type Actor%20Object%20Reference) (OtherComp :type Primitive%20Component%20Object%20Reference) (OtherBodyIndex :type Integer))
  (Utilities|Casting|CastToBP_ClassicBox OtherActor)
  (Variables|Default|SetbIsBlocked false)
  (Audio|Components|Audio|Stop (Variables|Default|GetStrongerHeat))
  (Rendering|Material|SetScalarParameterValueonMaterials (Variables|/Game/Core/ClassicObject/BP_ClassicBox.BP_ClassicBox_C|GetStaticMesh (stale OnComponentBeginOverlap(Box) _asbp_classic_box)) "StrongerEmissive" 0.0)
  (Rendering|Material|SetScalarParameterValueonMaterials (Variables|/Game/Core/ClassicObject/BP_ClassicBox.BP_ClassicBox_C|GetStaticMesh (stale OnComponentBeginOverlap(Box) _asbp_classic_box)) "Alpha" 0.0)
  (Niagara|SetNiagaraVariable(Vector3) (Variables|Default|GetNiagara) "Beam Start" (Math|Vector|MakeVector 1.5e+03 0.0 0.0)))

(event Custom|heat
  (bind (_direction _alpha _alphaforlerp) (Timeline|StrongerHeat PlayFromStart)
    (:Update
      (Rendering|Material|SetScalarParameterValueonMaterials (Variables|/Game/Core/ClassicObject/BP_ClassicBox.BP_ClassicBox_C|GetStaticMesh (stale OnComponentBeginOverlap(Box) _asbp_classic_box)) "StrongerEmissive" (Math|Float|Lerp 1.0 2.0 _alpha))
      (Rendering|Material|SetScalarParameterValueonMaterials (Variables|/Game/Core/ClassicObject/BP_ClassicBox.BP_ClassicBox_C|GetStaticMesh (stale OnComponentBeginOverlap(Box) _asbp_classic_box)) "Alpha" (Math|Float|Lerp 0.0 1.0 _alphaforlerp)))
    (:Finished
      (if (Math|Float|NearlyEqual(Float) _alpha 1.0 0.05)
        (bind _asbp_first_person_character (Utilities|Casting|CastToBP_FirstPersonCharacter (Game|Player|GetPlayerPawn 0)))
        (bind _grabbedactor (Variables|/Game/FirstPerson/Blueprints/BP_FirstPersonCharacter.BP_FirstPersonCharacter_C|GetgrabbedActor _asbp_first_person_character)
          (:then
            (Variables|/Game/FirstPerson/Blueprints/BP_FirstPersonCharacter.BP_FirstPersonCharacter_C|SetGrabbing _asbp_first_person_character false)
            (Physics|Components|PhysicsHandle|ReleaseComponent (Variables|/Game/FirstPerson/Blueprints/BP_FirstPersonCharacter.BP_FirstPersonCharacter_C|GetPhysicsHandle _asbp_first_person_character))
            (Actor|DestroyActor _grabbedactor)
            (Variables|/Game/FirstPerson/Blueprints/BP_FirstPersonCharacter.BP_FirstPersonCharacter_C|SetgrabbedActor _asbp_first_person_character 0))
          (:else
            _))
        (Default|Death _asbp_first_person_character (Variables|Default|GetVoiceline%20Row%20Name%20Explosion) false)
        (bind _outactors (Actor|GetAllActorsOfClass "BP_Laser_C"))
        (for _array_element _outactors
          (Variables|BP_Laser_C|SetbhasDiedExplosion? _array_element true))))))

(fn ConstructionScript)