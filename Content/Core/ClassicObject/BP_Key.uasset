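; BP_Key is a key pickup that the first-person player collects through an Interaction event.
; BeginPlay caches the player character, and interacting sets HasKey on the player passed in, then destroys the key.
; A key flagged IsTheOne also calls ModifyBlockedHealth on the player's subtitle reference and enables CanRemoveLock.
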(event Collision|EventActorBeginOverlap
  (params (OtherActor :type Actor%20Object%20Reference)))

(event EventTick
  (params (DeltaSeconds :type Float%20%28single-precision%29)))

(event EventInteraction
  (params (PlayerRef :type BP%20First%20Person%20Character%20Object%20Reference))
  (Variables|/Game/FirstPerson/Blueprints/BP_FirstPersonCharacter.BP_FirstPersonCharacter_C|SetbHasKey? PlayerRef true)
  (if (Variables|Default|GetbIsTheOne?)
    (Default|ModifyBlockedHealth (Variables|/Game/FirstPerson/Blueprints/BP_FirstPersonCharacter.BP_FirstPersonCharacter_C|GetSubtitleRef PlayerRef))
    (Variables|/Game/FirstPerson/Blueprints/BP_FirstPersonCharacter.BP_FirstPersonCharacter_C|SetbCanRemoveLock PlayerRef true))
  (Actor|DestroyActor))

(event EventBeginPlay
  (bind _asbp_first_person_character (Utilities|Casting|CastToBP_FirstPersonCharacter (Game|Player|GetPlayerPawn 0)))
  (Variables|Default|SetPlayerRef _asbp_first_person_character))

(fn ConstructionScript)