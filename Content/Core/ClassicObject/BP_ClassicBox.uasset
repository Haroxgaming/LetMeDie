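; BP_ClassicBox is a physics box the first-person player grabs and throws.
; Interaction attaches it to the player's PhysicsHandle and ignores Pawn collision; Throw restores blocking and adds a camera-forward impulse only when aiming upward.
; On overlap, a fast-falling box kills the player, releases any grab and tells every BP_SpawnButton to destroy its boxes.
; Otherwise, it breaks destructible windows when any positive velocity component exceeds a threshold.
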(event OnComponentBeginOverlap(Box)
  (params (OverlappedComponent :type Primitive%20Component%20Object%20Reference) (OtherActor :type Actor%20Object%20Reference) (OtherComp :type Primitive%20Component%20Object%20Reference) (OtherBodyIndex :type Integer) (bFromSweep :type Boolean) (SweepResult :type Hit%20Result%20Structure%20%28by%20ref%29))
  (bind _returnvalue (Transformation|GetVelocity))
  (bind (_x _y _z) (Math|Vector|BreakVector _returnvalue))
  (if (not (Variables|Default|GetbHasDied?))
    (bind _asbp_first_person_character (Utilities|Casting|CastToBP_FirstPersonCharacter OtherActor)
      (:then
        (if (<= (.Z (Math|Vector|BreakVector (Transformation|GetComponentVelocity (Variables|Default|GetBox)))) -5e+02)
          (Default|Death _asbp_first_person_character "None" false)
          (CallFunction|KillEvent)
          (if (Variables|/Game/FirstPerson/Blueprints/BP_FirstPersonCharacter.BP_FirstPersonCharacter_C|GetGrabbing _asbp_first_person_character)
            (Physics|Components|PhysicsHandle|ReleaseComponent (Variables|/Game/FirstPerson/Blueprints/BP_FirstPersonCharacter.BP_FirstPersonCharacter_C|GetPhysicsHandle _asbp_first_person_character))
            (Variables|/Game/FirstPerson/Blueprints/BP_FirstPersonCharacter.BP_FirstPersonCharacter_C|SetgrabbedActor _asbp_first_person_character 0)
            (Variables|/Game/FirstPerson/Blueprints/BP_FirstPersonCharacter.BP_FirstPersonCharacter_C|SetGrabbing _asbp_first_person_character false))
          (bind _outactors (Actor|GetAllActorsOfClass "/Game/Core/ClassicObject/BP_SpawnButton.BP_SpawnButton_C"))
          (for _array_element _outactors
            (Variables|/Game/Core/ClassicObject/BP_SpawnButton.BP_SpawnButton_C|SetDeath%20? _array_element true)
            (Default|DestroyBoxes _array_element))))
      (:CastFailed
        (bind _asbp_destructible_window (Utilities|Casting|CastToBP_DestructibleWindow OtherActor :!label _label))
        (if (Math|Boolean|ORBoolean (> _x 3e+02) (> _y 3e+02) (> _z 3e+02))
          (Default|Breaking _asbp_destructible_window))))
    (else
      (goto _label))))

(event EventBeginPlay
  (|CallParentFunction))

(event EventThrow
  (params (PlayerRef :type BP%20First%20Person%20Character%20Object%20Reference))
  (bind _firstpersoncamera (Variables|/Game/FirstPerson/Blueprints/BP_FirstPersonCharacter.BP_FirstPersonCharacter_C|GetFirstPersonCamera PlayerRef))
  (bind _relativerotation (Variables|/Script/Engine.SceneComponent|GetRelativeRotation _firstpersoncamera))
  (Development|PrintString "box throw" true false)
  (Variables|/Game/FirstPerson/Blueprints/BP_FirstPersonCharacter.BP_FirstPersonCharacter_C|SetGrabbing PlayerRef false)
  (Physics|Components|PhysicsHandle|ReleaseComponent (Variables|/Game/FirstPerson/Blueprints/BP_FirstPersonCharacter.BP_FirstPersonCharacter_C|GetPhysicsHandle PlayerRef))
  (Collision|SetCollisionResponsetoChannel (Variables|Default|GetStaticMesh) "ECC_Pawn" "ECR_Block")
  (Development|PrintString (Utilities|String|ToString(Float) (.pitch _relativerotation)) true false)
  (if (> (.pitch _relativerotation) 1e+01)
    (Physics|AddImpulse (Variables|Default|GetBox) (* (Math|Vector|GetForwardVector _firstpersoncamera) 1e+03) "None" true)))

(event EventInteraction
  (params (PlayerRef :type BP%20First%20Person%20Character%20Object%20Reference))
  (bind _self self)
  (if (not (Variables|/Game/FirstPerson/Blueprints/BP_FirstPersonCharacter.BP_FirstPersonCharacter_C|GetGrabbing PlayerRef))
    (Development|PrintString (Utilities|GetDisplayName _self) true false)
    (Variables|/Game/FirstPerson/Blueprints/BP_FirstPersonCharacter.BP_FirstPersonCharacter_C|SetgrabbedActor PlayerRef _self)
    (Variables|/Game/FirstPerson/Blueprints/BP_FirstPersonCharacter.BP_FirstPersonCharacter_C|SetGrabbing PlayerRef true)
    (Class|PhysicsHandleComponent|GrabComponentatLocation (Variables|/Game/FirstPerson/Blueprints/BP_FirstPersonCharacter.BP_FirstPersonCharacter_C|GetPhysicsHandle PlayerRef) (Variables|Default|GetBox) "Scene" (Transformation|GetActorLocation))
    (Collision|SetCollisionResponsetoChannel (Variables|Default|GetStaticMesh) "ECC_Pawn" "ECR_Ignore")))

(fn ConstructionScript
  (|CallParentFunction))