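; BP_button is an interactable monitor button that either opens an electricity minigame or moves a linked platform.
; With HasMiniGame set, Interaction creates WBP_ElectricityWidget, passing itself and a death flag; otherwise it calls Moving on the standard or size power-up platform.
; The construction script picks monitor materials by mode.
; In minigame mode, a self-restarting timer randomizes a material parameter at random intervals until CancelMats clears it.
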(event Custom|ChangeValue
  (bind _output_get (Variables|Default|SetTempTimer (Math|Random|RandomFloatinRange 1.0 3.0)))
  (Rendering|Material|SetScalarParameterValueonMaterials (Variables|Default|GetMonitor) "RandomValue" _output_get)
  (bind _returnvalue (Utilities|Time|SetTimerbyEvent (delegate Custom|ChangeValue) _output_get))
  (Variables|Default|SetNewVar _returnvalue))

(event Custom|CancelMats
  (Utilities|Time|ClearandInvalidateTimerbyHandle (Variables|Default|GetNewVar)))

(event EventBeginPlay
  (if (Variables|Default|GetbHasMiniGame?)
    (bind _output_get (Variables|Default|SetTempTimer (Math|Random|RandomFloatinRange 1.0 3.0)))
    (Rendering|Material|SetScalarParameterValueonMaterials (Variables|Default|GetMonitor) "RandomValue" _output_get)
    (bind _returnvalue (Utilities|Time|SetTimerbyEvent (delegate Custom|ChangeValue) _output_get))
    (Variables|Default|SetNewVar _returnvalue)))

(event EventInteraction
  (params (PlayerRef :type BP%20First%20Person%20Character%20Object%20Reference))
  (bind _movingplatform (Variables|Default|GetMovingPlatform))
  (if (Variables|Default|GetbHasMiniGame?)
    (bind _returnvalue (UserInterface|CreateWidget "/Game/Core/UI/Widgets/WBP_ElectricityWidget.WBP_ElectricityWidget_C" 0 (Variables|Default|GetbElectricityDeath?) self))
    (UserInterface|Viewport|AddtoViewport _returnvalue 0)
    (elif (Variables|Default|GetbIsPowerUPone?)
      (bind _asbp_moving_platform_with_size_power_up (Utilities|Casting|CastToBP_MovingPlatformWithSizePowerUP _movingplatform))
      (Default|Moving _asbp_moving_platform_with_size_power_up)
      (else
        (bind _asbp_moving_platform (Utilities|Casting|CastToBP_MovingPlatform _movingplatform))
        (Default|Moving _asbp_moving_platform)))))

(fn ConstructionScript
  (bind _monitor (Variables|Default|GetMonitor))
  (if (Variables|Default|GetbHasMiniGame?)
    (Rendering|Material|SetMaterial _monitor 1 "/Game/Core/Materials/M_Panner.M_Panner")
    (else
      (Rendering|Material|SetMaterial _monitor 1 "/Game/ScienceLab/Materials/OfficeProps/MI_Office_Monitor.MI_Office_Monitor")
      (Rendering|Material|SetMaterial _monitor 2 "/Game/ScienceLab/Materials/OfficeProps/MI_Office_Monitor.MI_Office_Monitor"))))