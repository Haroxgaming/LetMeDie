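; BP_Wall is a configurable wall actor with all its logic in the construction script; its event graph is unused.
; Boolean options swap both wall meshes to a windowed or piped variant, with windowed taking priority over piped.
; A separate barrierless option destroys two additional static mesh components, independent of the chosen wall variant.
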(event EventBeginPlay)

(event Collision|EventActorBeginOverlap
  (params (OtherActor :type Actor%20Object%20Reference)))

(event EventTick
  (params (DeltaSeconds :type Float%20%28single-precision%29)))

(fn ConstructionScript
  (if (Variables|Default|GetbIsWindowed?)
    (Components|StaticMesh|SetStaticMesh (Variables|Default|Getwall1) "/Game/Core/Map/_GENERATED/EDUSERVICES/SM_WindowedWall.SM_WindowedWall")
    (Components|StaticMesh|SetStaticMesh (Variables|Default|Getwall0) "/Game/Core/Map/_GENERATED/EDUSERVICES/SM_WindowedWall.SM_WindowedWall")
    (elif (Variables|Default|Getb_IsPipedWall)
      (Components|StaticMesh|SetStaticMesh (Variables|Default|Getwall1) "/Game/Core/Map/_GENERATED/EDUSERVICES/SM_PipedWall.SM_PipedWall")
      (Components|StaticMesh|SetStaticMesh (Variables|Default|Getwall0) "/Game/Core/Map/_GENERATED/EDUSERVICES/SM_PipedWall.SM_PipedWall")))
  (if (Variables|Default|GetbIsBarrierLess?)
    (Components|DestroyComponent (Variables|Default|GetStaticMesh))))