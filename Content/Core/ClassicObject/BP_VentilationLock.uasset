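; Ventilation lock actor that kills the first-person player who enters its trigger box while carrying a classic box.
; On overlap it releases the player's physics-handle grab, teleports the box to its Scene component, disables the box's physics and mesh collision, then calls Death with a configurable voiceline row.
; A timer then removes the box from the linked button's ClassicBoxRef collection and destroys it.
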(event OnComponentBeginOverlap(Box)
  (params (OverlappedComponent :type Primitive%20Component%20Object%20Reference) (OtherActor :type Actor%20Object%20Reference) (OtherComp :type Primitive%20Component%20Object%20Reference) (OtherBodyIndex :type Integer) (bFromSweep :type Boolean) (SweepResult :type Hit%20Result%20Structure%20%28by%20ref%29))
  (bind _asbp_first_person_character (Utilities|Casting|CastToBP_FirstPersonCharacter OtherActor))
  (bind _asbp_classic_box (Utilities|Casting|CastToBP_ClassicBox (Variables|/Game/FirstPerson/Blueprints/BP_FirstPersonCharacter.BP_FirstPersonCharacter_C|GetgrabbedActor _asbp_first_person_character)))
  (Physics|Components|PhysicsHandle|ReleaseComponent (Variables|/Game/FirstPerson/Blueprints/BP_FirstPersonCharacter.BP_FirstPersonCharacter_C|GetPhysicsHandle _asbp_first_person_character))
  (Variables|/Game/FirstPerson/Blueprints/BP_FirstPersonCharacter.BP_FirstPersonCharacter_C|SetGrabbing _asbp_first_person_character false)
  (Transformation|SetActorLocation _asbp_classic_box (Transformation|GetWorldLocation (Variables|Default|GetScene)) false false)
  (Physics|SetSimulatePhysics (Variables|/Game/Core/ClassicObject/BP_ClassicBox.BP_ClassicBox_C|GetStaticMesh _asbp_classic_box) false)
  (Collision|SetCollisionResponsetoAllChannels (Variables|/Game/Core/ClassicObject/BP_ClassicBox.BP_ClassicBox_C|GetStaticMesh _asbp_classic_box) "ECR_Ignore")
  (Default|Death _asbp_first_person_character (Variables|Default|GetVoiceline%20Row%20Name) false)
  (Utilities|Time|SetTimerbyEvent (delegate Custom|CustomEvent) 2.0))

(event Custom|CustomEvent
  (Utilities|Array|RemoveItem (Variables|/Game/Core/ClassicObject/BP_SpawnButton.BP_SpawnButton_C|GetClassicBoxRef (Variables|Default|GetBP_Button)) (stale OnComponentBeginOverlap(Box) _asbp_classic_box))
  (Actor|DestroyActor (stale OnComponentBeginOverlap(Box) _asbp_classic_box)))

(event EventBeginPlay)

(event Collision|EventActorBeginOverlap
  (params (OtherActor :type Actor%20Object%20Reference)))

(event EventTick
  (params (DeltaSeconds :type Float%20%28single-precision%29)))

(fn ConstructionScript)