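; BP_Door is a two-panel sliding door that opens for the player, serving as checkpoint, tutorial cue and game ending.
; When unlocked, its Box overlaps save the player's checkpoint and drive the OpenClose timeline forward or back.
; IsLocked selects a different mesh at construction and blocks opening until Unlock is called.
; IsFirstDoor runs a timed voiceline reminder until first overlap, while IsLastDoor shows credits instead of opening.
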(event OnComponentBeginOverlap(Box)
  (params (OverlappedComponent :type Primitive%20Component%20Object%20Reference) (OtherActor :type Actor%20Object%20Reference) (OtherComp :type Primitive%20Component%20Object%20Reference) (OtherBodyIndex :type Integer) (bFromSweep :type Boolean) (SweepResult :type Hit%20Result%20Structure%20%28by%20ref%29))
  (bind _newvar (Variables|Default|GetNewVar))
  (bind _asbp_first_person_character (Utilities|Casting|CastToBP_FirstPersonCharacter OtherActor))
  (if (Utilities|Time|IsValidTimerHandle _newvar)
    (Utilities|Time|ClearandInvalidateTimerbyHandle _newvar)
    (Default|DialogueAnimation (Variables|/Game/FirstPerson/Blueprints/BP_FirstPersonCharacter.BP_FirstPersonCharacter_C|GetSubtitleRef (.AsBP%20First%20Person%20Character (Utilities|Casting|CastToBP_FirstPersonCharacter (Game|Player|GetPlayerPawn 0)))) "TutoEntrance" 1.0))
  (if (not (Variables|Default|GetbIsLocked?))
    (Variables|/Game/FirstPerson/Blueprints/BP_FirstPersonCharacter.BP_FirstPersonCharacter_C|SetCheckpoint _asbp_first_person_character (Transformation|GetActorLocation _asbp_first_person_character))
    (if (Variables|Default|GetbIsLastDoor)
      (Default|DialogueAnimation (Variables|/Game/FirstPerson/Blueprints/BP_FirstPersonCharacter.BP_FirstPersonCharacter_C|GetSubtitleRef _asbp_first_person_character) "None" 0.0)
      (Utilities|FlowControl|Delay 1e+01)
      (Widget|RemovefromParent (Variables|/Game/FirstPerson/Blueprints/BP_FirstPersonCharacter.BP_FirstPersonCharacter_C|GetSubtitleRef _asbp_first_person_character))
      (bind _returnvalue (UserInterface|CreateWidget "/Game/Core/UI/Widgets/WBP_Credits.WBP_Credits_C"))
      (UserInterface|Viewport|AddtoViewport _returnvalue 0)
      (else
        (bind _alpha (Timeline|Open/Close Play)
          (:Update
            (Transformation|SetRelativeLocation (Variables|Default|GetDoor) (select (Variables|Default|GetbIsLocked?) (Math|Vector|Lerp(Vector) "20.000000,0.000000,-10.000000" "20.000000,120.000000,-10.000000" _alpha) (Math|Vector|Lerp(Vector) "20.000000,0.000000,0.000000" "20.000000,120.000000,0.000000" _alpha)) false false)
            (Transformation|SetRelativeLocation (Variables|Default|GetDoor1) (select (Variables|Default|GetbIsLocked?) (Math|Vector|Lerp(Vector) "-20.000000,0.000000,-10.000000" "-20.000000,120.000000,-10.000000" _alpha) (Math|Vector|Lerp(Vector) "-20.000000,0.000000,0.000000" "-20.000000,120.000000,0.000000" _alpha)) false false)))))))

(event OnComponentEndOverlap(Box)
  (params (OverlappedComponent :type Primitive%20Component%20Object%20Reference) (OtherActor :type Actor%20Object%20Reference) (OtherComp :type Primitive%20Component%20Object%20Reference) (OtherBodyIndex :type Integer))
  (bind _asbp_first_person_character (Utilities|Casting|CastToBP_FirstPersonCharacter OtherActor))
  (if (not (Variables|Default|GetbIsLocked?))
    (Variables|/Game/FirstPerson/Blueprints/BP_FirstPersonCharacter.BP_FirstPersonCharacter_C|SetCheckpoint _asbp_first_person_character (Transformation|GetActorLocation _asbp_first_person_character))
    (bind _alpha (Timeline|Open/Close Reverse)
      (:Update
        (Transformation|SetRelativeLocation (Variables|Default|GetDoor) (select (Variables|Default|GetbIsLocked?) (Math|Vector|Lerp(Vector) "20.000000,0.000000,-10.000000" "20.000000,120.000000,-10.000000" _alpha) (Math|Vector|Lerp(Vector) "20.000000,0.000000,0.000000" "20.000000,120.000000,0.000000" _alpha)) false false)
        (Transformation|SetRelativeLocation (Variables|Default|GetDoor1) (select (Variables|Default|GetbIsLocked?) (Math|Vector|Lerp(Vector) "-20.000000,0.000000,-10.000000" "-20.000000,120.000000,-10.000000" _alpha) (Math|Vector|Lerp(Vector) "-20.000000,0.000000,0.000000" "-20.000000,120.000000,0.000000" _alpha)) false false)))))

(event Custom|Unlock
  (params (PlayerRef :type BP%20First%20Person%20Character%20Object%20Reference))
  (Variables|Default|SetbIsLocked? false)
  (Variables|/Game/FirstPerson/Blueprints/BP_FirstPersonCharacter.BP_FirstPersonCharacter_C|SetCheckpoint PlayerRef (Transformation|GetActorLocation PlayerRef))
  (if (!= (Utilities|Array|FindItem (Collision|GetOverlappingActors (Variables|Default|GetBox) 0 :!class /Script/Engine.PrimitiveComponent) PlayerRef) -1)
    (bind _alpha (Timeline|Open/Close Play)
      (:Update
        (Transformation|SetRelativeLocation (Variables|Default|GetDoor) (select (Variables|Default|GetbIsLocked?) (Math|Vector|Lerp(Vector) "20.000000,0.000000,-10.000000" "20.000000,120.000000,-10.000000" _alpha) (Math|Vector|Lerp(Vector) "20.000000,0.000000,0.000000" "20.000000,120.000000,0.000000" _alpha)) false false)
        (Transformation|SetRelativeLocation (Variables|Default|GetDoor1) (select (Variables|Default|GetbIsLocked?) (Math|Vector|Lerp(Vector) "-20.000000,0.000000,-10.000000" "-20.000000,120.000000,-10.000000" _alpha) (Math|Vector|Lerp(Vector) "-20.000000,0.000000,0.000000" "-20.000000,120.000000,0.000000" _alpha)) false false)))))

(event Custom|DoorVoiceline
  (Default|DialogueAnimation (Variables|/Game/FirstPerson/Blueprints/BP_FirstPersonCharacter.BP_FirstPersonCharacter_C|GetSubtitleRef (.AsBP%20First%20Person%20Character (Utilities|Casting|CastToBP_FirstPersonCharacter (Game|Player|GetPlayerPawn 0)))) "IntroDoor" 1.0))

(event EventBeginPlay
  (Components|Timeline|SetPlayRate (Variables|Default|GetOpen/Close) (/ 1.0 (Variables|Default|GetPlayRate%28s%29)))
  (if (Variables|Default|GetbIsFirstDoor?)
    (bind _returnvalue (Utilities|Time|SetTimerbyEvent (delegate Custom|DoorVoiceline) 3e+01))
    (Variables|Default|SetNewVar _returnvalue)))

(fn ConstructionScript
  (bind _door1 (Variables|Default|GetDoor1))
  (bind _door (Variables|Default|GetDoor))
  (if (Variables|Default|GetbIsLocked?)
    (Components|StaticMesh|SetStaticMesh (Variables|Default|GetDoor) "/Game/ScienceLab/Meshes/Rooms/Doors/SM_LabDoor04.SM_LabDoor04")
    (Components|StaticMesh|SetStaticMesh (Variables|Default|GetDoor1) "/Game/ScienceLab/Meshes/Rooms/Doors/SM_LabDoor04.SM_LabDoor04")
    (Transformation|SetRelativeScale3D _door "1.200000,1.200000,1.200000")
    (Transformation|SetRelativeLocation _door (- (Variables|/Script/Engine.SceneComponent|GetRelativeLocation _door) "0.000000,0.000000,10.000000") false false)
    (Transformation|SetRelativeLocation _door1 (- (Variables|/Script/Engine.SceneComponent|GetRelativeLocation _door1) "0.000000,0.000000,10.000000") false false)))