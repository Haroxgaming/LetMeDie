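; Moving platform that toggles between up and down locations and spawns a BP_SizeBuff power-up on top of itself.
; A Light timeline ramps a RectLight over the cooldown, then spawns the buff with a reference back to the platform.
; The Moving event lerps the platform and buff via timeline, flipping IsUp when finished.
; Player overlap during descent triggers Death and clears NotDead on all platforms of both moving-platform classes, blocking repeat kills.
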(event OnComponentBeginOverlap(Box)
  (params (OverlappedComponent :type Primitive%20Component%20Object%20Reference) (OtherActor :type Actor%20Object%20Reference) (OtherComp :type Primitive%20Component%20Object%20Reference) (OtherBodyIndex :type Integer) (bFromSweep :type Boolean) (SweepResult :type Hit%20Result%20Structure%20%28by%20ref%29))
  (bind _asbp_first_person_character (Utilities|Casting|CastToBP_FirstPersonCharacter OtherActor))
  (if (Math|Boolean|ANDBoolean (Audio|Components|Audio|IsPlaying (Variables|Default|GetMovingDown/Up)) (Variables|Default|GetbIsUp?) (Variables|Default|GetbNotDead?))
    (Default|Death _asbp_first_person_character "None" false 0.0 0.0)
    (Variables|Default|SetbNotDead? false)
    (bind _outactors (Actor|GetAllActorsOfClass "/Game/Core/ClassicObject/BP_MovingPlatform.BP_MovingPlatform_C"))
    (for _array_element _outactors
      (Variables|/Game/Core/ClassicObject/BP_MovingPlatform.BP_MovingPlatform_C|SetNotDead _array_element false))
    (bind _outactors_2 (Actor|GetAllActorsOfClass "BP_MovingPlatformWithSizePowerUP_C"))
    (for _array_element_2 _outactors_2
      (Variables|BP_MovingPlatformWithSizePowerUP_C|SetbNotDead? _array_element_2 false))))

(event Custom|Moving
  (bind _newvar (Variables|Default|GetNewVar))
  ;[0.15 0.15 0.15 0.5] Moving
  (if (not (Audio|Components|Audio|IsPlaying (Variables|Default|GetMovingDown/Up)))
    (Variables|Default|SetbaseLoc (Transformation|GetActorLocation))
    (bind _alpha (Timeline|MovingDown/Up PlayFromStart)
      (:Update
        (Transformation|SetActorLocation (Math|Vector|Lerp(Vector) (Variables|Default|GetbaseLoc) (Math|Vector|SelectVector (Variables|Default|GetDownLoc) (Variables|Default|GetUpLoc) (Variables|Default|GetbIsUp?)) _alpha) false false)
        (Utilities|IsValid _newvar
          (:Is%20Valid
            (Transformation|SetActorLocation _newvar (+ (Math|Vector|Lerp(Vector) (Variables|Default|GetbaseLoc) (Math|Vector|SelectVector (Variables|Default|GetDownLoc) (Variables|Default|GetUpLoc) (Variables|Default|GetbIsUp?)) _alpha) "0.000000,0.000000,100.000000") false false))))
      (:Finished
        (Variables|Default|SetbIsUp? (not (Variables|Default|GetbIsUp?)))))))

(event Custom|SpawnPowerUP
  (bind _rectlight (Variables|Default|GetRectLight))
  ;[0.15 0.15 0.15 0.5] PowerUP
  (bind _alpha (Timeline|Light Play)
    (:Update
      (Rendering|Components|Light|SetIntensity _rectlight (Math|Float|Lerp 0.0 1e+03 _alpha)))
    (:Finished
      (bind _returnvalue (Game|SpawnActorfromClass "/Game/Core/Death/BP_SizeBuff.BP_SizeBuff_C" (Math|Transform|MakeTransform (+ (Transformation|GetWorldLocation (Variables|Default|GetStaticMesh1)) "0.000000,0.000000,50.000000") "0, 0, 0" "1.000000,1.000000,1.000000") "AdjustIfPossibleButAlwaysSpawn" "MultiplyWithRoot" 0 self 0))
      (Variables|Default|SetNewVar _returnvalue)
      (Rendering|Components|Light|SetIntensity _rectlight 0.0))))

(event EventBeginPlay
  ;[0.15 0.15 0.15 0.5] Initialiasing PlayRate
  (Components|Timeline|SetPlayRate (Variables|Default|GetMovingDown/Up) (/ 1.0 (Variables|Default|GetMovementPlayRate%28s%29)))
  (Variables|Default|SetUpLoc (Transformation|GetActorLocation))
  (Components|Timeline|SetPlayRate (Variables|Default|GetLight) (/ 1.0 (Variables|Default|GetSpawnCooldown%28s%29)))
  (CallFunction|SpawnPowerUP))

(fn ConstructionScript)