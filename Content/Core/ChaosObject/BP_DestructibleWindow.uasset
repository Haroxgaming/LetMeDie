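; BP_DestructibleWindow is a window actor that shatters once when its Breaking event is called.
; Breaking plays the Glassbreaking subtitle dialogue, swaps the intact mesh for a physics-simulated broken one and applies a radial impulse.
; After a short delay, it loosens collision and pushes the debris backward along the Arrow.
; Rebuild restores the intact look, Cube blocking and start location but destroys the broken component without resetting DoOnce.
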(event Custom|Breaking
  (bind _brokenwindow (Variables|Default|GetBrokenWindow))
  (bind _brokenwindow_2 (Variables|Default|GetBrokenWindow))
  (Utilities|FlowControl|DoOnce false
    (:Completed
      (Default|DialogueAnimation (Variables|/Game/FirstPerson/Blueprints/BP_FirstPersonCharacter.BP_FirstPersonCharacter_C|GetSubtitleRef (.AsBP%20First%20Person%20Character (Utilities|Casting|CastToBP_FirstPersonCharacter (Game|Player|GetPlayerPawn 0)))) "Glassbreaking" 1.0)
      (Rendering|SetVisibility (Variables|Default|GetWindow) false false)
      (Rendering|SetVisibility _brokenwindow_2 true false)
      (Physics|SetSimulatePhysics _brokenwindow_2 true)
      (Class|PhysicsObjectBlueprintLibrary|ApplyRadialImpulse _brokenwindow (Transformation|GetWorldLocation _brokenwindow) 5e+01 5e+02 "RIF_Constant" false 0.0 true 0.0 1.0)
      (Utilities|FlowControl|Delay 0.15)
      (Collision|SetCollisionResponsetoAllChannels (Variables|Default|GetCube) "ECR_Ignore")
      (Physics|AddImpulse _brokenwindow_2 (* (Math|Vector|GetForwardVector (Variables|Default|GetArrow)) -2e+03) "None" true)
      (Collision|SetCollisionResponsetoAllChannels (Variables|Default|GetSM_Window) "ECR_Ignore")
      (Collision|SetCollisionResponsetoAllChannels (Variables|Default|GetBrokenWindow) "ECR_Overlap"))))

(event Custom|rebuild
  (Collision|SetCollisionResponsetoAllChannels (Variables|Default|GetCube) "ECR_Block")
  (Rendering|SetVisibility (Variables|Default|GetWindow) true false)
  (Rendering|SetVisibility (Variables|Default|GetBrokenWindow) false false)
  (Components|DestroyComponent (Variables|Default|GetBrokenWindow))
  (Transformation|SetActorLocation (Variables|Default|GetBeginLoc) false false))

(event EventBeginPlay
  (Variables|Default|SetBeginLoc (Transformation|GetActorLocation)))

(fn ConstructionScript)