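; BP_Wire01 is a configurable wire actor that builds spline meshes along its Spline in the construction script.
; SplineMeshVar chooses one segment per point pair or segments at fixed Spacing with scaled direction tangents.
; WireVar picks among six spline mesh components, three of which take a second material slot.
; Each segment is scaled by WireSize and gets dynamic MI_Wire instances driven by color, dirt, roughness, specular and TextureVar texture sets.
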(fn ConstructionScript
  (|Wire))